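; Heads-up display Blueprint that holds camera tab state and owns the reference to a LocalGovActor.
; On BeginPlay it spawns the LocalGovActor and exposes it through GetLocalGovReference.
; SetCamTab stores the tab value and clears the shifted flag, MarkCamChanged sets it, and GetChangedVal reports both.
; MoveCamera is a stub with no camera logic.
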(event EventBeginPlay
  (bind _returnvalue (Game|SpawnActorfromClass "/Script/FinalHUDTest.LocalGovActor" (Math|Transform|MakeTransform "0, 0, 0" "0, 0, 0" "1,1,1") "Undefined" 0 0))
  (Variables|Default|SetLocalGov _returnvalue))

(event Collision|EventActorBeginOverlap
  (params (OtherActor :type Actor%20Object%20Reference)))

(event EventSetCamTab
  (params (TabVal :type Integer))
  (Variables|Default|SetTabVal TabVal)
  (Variables|Default|SetCameraShifted false))

(event EventMarkCamChanged
  (Variables|Default|SetCameraShifted true))

(event EventTick
  (params (DeltaSeconds :type Float%20%28single-precision%29)))

(fn ConstructionScript)

(fn GetChangedVal
  (return (Variables|Default|GetCameraShifted) (Variables|Default|GetTabVal)))

(fn GetLocalGovReference
  (return (Variables|Default|GetLocalGov)))

(fn MoveCamera
  (params (LocationIndex :type Integer))
  (return 0))